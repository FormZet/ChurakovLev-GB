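; Save/load state controller for the Collaborative Viewer that connects the persistent UI menu to named save slots.
; A one-time init from the player controller loads the MainSaveGame name index, or creates one plus a data save for the first menu option.
; It fills the load-state options from the saved names and binds menu events.
; Save and load handlers delegate to the pawn's SaveLoadState through its ROS save-game functions.
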(event `BeginPlayFromController`
  (`/Engine/EditorBlueprintResources/StandardMacros.DoOnce` false
    (:`Completed`
      (bind _asbp_collab_v_player_controller (cast `/Game/Imported/CollaborativeViewer/Blueprints/PlayerController/BP_Collab_V_PlayerController` (`GameplayStatics.GetPlayerController` 0)))
      (set `self.Persistent_UI` (`/Game/Imported/CollaborativeViewer/Blueprints/PlayerController/BP_Collab_V_PlayerController.Persistent_UI` _asbp_collab_v_player_controller))
      (`self.CreateMainSlot_SaveGame`)
      (`self.MainSaveGameToPersistentMenu`)
      (`self.BindToMenu`))))

(event `BindToMenu`
  (bind _asbp_collab_v_player_controller (cast `/Game/Imported/CollaborativeViewer/Blueprints/PlayerController/BP_Collab_V_PlayerController` (`GameplayStatics.GetPlayerController` 0)))
  (bind _persistent_ui (`/Game/Imported/CollaborativeViewer/Blueprints/PlayerController/BP_Collab_V_PlayerController.Persistent_UI` _asbp_collab_v_player_controller))
  (add `/Game/Imported/CollaborativeViewer/UMG/GameMenu/Persistent_ToolBar.SavingState` _persistent_ui (`|CreateDelegate` :!event `AddToMainSveGame`))
  (add `/Game/Imported/CollaborativeViewer/UMG/GameMenu/Persistent_ToolBar.LoadState` _persistent_ui (`|CreateDelegate` :!event `LoadSaveGame`)))

(event `AddToMainSveGame`
  (params (SlotName :type "String (by ref)"))
  (bind _asbp_base_pawn (cast `/Game/Imported/CollaborativeViewer/Blueprints/Pawn/BP_BasePawn` (`GameplayStatics.GetPlayerPawn` 0)))
  (`/Game/Imported/CollaborativeViewer/Blueprints/SaveGame/SaveLoad_State_Pawn.SaveGameROS` (`/Game/Imported/CollaborativeViewer/Blueprints/Pawn/BP_BasePawn.SaveLoad_State` _asbp_base_pawn) SlotName (`self.SaveGame`)))

(event `LoadSaveGame`
  (params (Option :type String) (SaveGameMain :type "/Game/Imported/CollaborativeViewer/Blueprints/SaveGame/BP_Data_SaveGame Object Reference"))
  (bind _asbp_base_pawn (cast `/Game/Imported/CollaborativeViewer/Blueprints/Pawn/BP_BasePawn` (`GameplayStatics.GetPlayerPawn` 0)))
  (`/Game/Imported/CollaborativeViewer/Blueprints/SaveGame/SaveLoad_State_Pawn.LoadSaveGameROS` (`/Game/Imported/CollaborativeViewer/Blueprints/Pawn/BP_BasePawn.SaveLoad_State` _asbp_base_pawn) Option SaveGameMain))

(event `MainSaveGameToPersistentMenu`
  (for _array_element (`/Game/Imported/CollaborativeViewer/Blueprints/SaveGame/BP_Name_SaveGame.SaveGameNameArray` (`self.SaveGame`))
    (`ComboBoxString.AddOption` (`/Game/Imported/CollaborativeViewer/UMG/GameMenu/Persistent_ToolBar.Load_State` (`self.Persistent_UI`)) _array_element)))

(event `CreateMainSlot_SaveGame`
  (if (`BlueprintPathsLibrary.FileExists` (`KismetStringLibrary.Concat_StrStr` (`KismetSystemLibrary.GetProjectSavedDirectory`) "SaveGames/MainSaveGame.sav"))
    (bind _returnvalue (`GameplayStatics.LoadGameFromSlot` "MainSaveGame"))
    (bind _asbp_name_save_game (cast `/Game/Imported/CollaborativeViewer/Blueprints/SaveGame/BP_Name_SaveGame` _returnvalue))
    (set `self.SaveGame` _asbp_name_save_game)
    (else
      (bind _returnvalue_2 (`GameplayStatics.CreateSaveGameObject` "/Game/Imported/CollaborativeViewer/Blueprints/SaveGame/BP_Name_SaveGame.BP_Name_SaveGame_C"))
      (set `self.SaveGame` _returnvalue_2)
      (bind _returnvalue_3 (`GameplayStatics.CreateSaveGameObject` "/Game/Imported/CollaborativeViewer/Blueprints/SaveGame/BP_Data_SaveGame.BP_Data_SaveGame_C"))
      (`GameplayStatics.SaveGameToSlot` _returnvalue_3 (`ComboBoxString.GetOptionAtIndex` (`/Game/Imported/CollaborativeViewer/UMG/GameMenu/Persistent_ToolBar.Load_State` (`self.Persistent_UI`)) 0)))))